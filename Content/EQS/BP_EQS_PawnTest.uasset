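; Test pawn for trying out Environment Query System queries through its AI controller.
; On BeginPlay a looping timer runs the QueryTest query every two seconds in random-best-25% mode and draws a green debug sphere at each successful result location.
; Unconnected debug chains print sight angle, behind check and distance-based score against the player character, but none of them run.
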(event `self.ReceiveBeginPlay`
  (`KismetSystemLibrary.K2_SetTimerDelegate` (delegate `Query`) 2.0 true))

(event `Query`
  (bind (_asynctaskproxy _location) (`RunEQSQuery_Task.RunEQSQuery_Task` (`AIBlueprintHelperLibrary.GetAIController` self) (`self.QueryTest`) (`self.In Query Config`) "RandomBest25Pct")
    (:`OnSuccess`
      (`KismetSystemLibrary.DrawDebugSphere` _location 100.0 12 (struct :`R` 0.070435 :`G` 1.0 :`B` 0.006243 :`A` 1.0) 2.0 5.0))))

(fn `UserConstructionScript`)