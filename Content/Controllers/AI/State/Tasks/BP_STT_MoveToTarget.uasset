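; StateTree task that moves an AI controller's pawn to its current target actor.
; On latent enter, it gets the target from the controller context, sets focus on it and runs AI MoveTo with the configured acceptance radius.
; The task succeeds when the move finishes and fails when the request fails; an invalid target leaves it without a finish call.
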(event `self.ReceiveLatentEnterState`
  (params (Transition :type "StateTreeTransitionResult Structure (by ref)"))
  (bind _returnvalue (message `EnemyControlInterface.GetTargetActor` (`self.ControllerContext`)))
  (`/Engine/EditorBlueprintResources/StandardMacros.IsValid` _returnvalue
    (:`Is Valid`
      (`AIController.K2_SetFocus` (`self.ControllerContext`) _returnvalue)
      (`AITask_MoveTo.AIMoveTo` (`self.ControllerContext`) (`Actor.K2_GetActorLocation` _returnvalue) _returnvalue (`self.AcceptanceRadius`)
        (:`OnRequestFailed`
          (`self.FinishTask` false))
        (:`OnMoveFinished`
          (`self.FinishTask` true))))))