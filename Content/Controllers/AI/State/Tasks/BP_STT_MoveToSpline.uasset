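; StateTree task that moves an AI-controlled pawn toward a target actor along a spawned zig-zag spline.
; On enter it spawns BP_ZigZagSpline aimed at the target and sends the pawn an acceleration message.
; From tick, it focuses on and moves to each spline point in turn, then destroys the spline and succeeds.
; Failures restore normal movement and, if the spline exists, destroy it and fail the task.
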(event `self.ReceiveLatentEnterState`
  (params (Transition :type "StateTreeTransitionResult Structure (by ref)"))
  (bind _controllercontext (`self.ControllerContext`))
  (bind _targetactor (`self.TargetActor`))
  (bind _returnvalue (`Actor.K2_GetActorLocation` _controllercontext))
  (`self.SplineActor`
    (:`then`)
    (:`else`
      (bind _targetactor_2 (`self.TargetActor`)
        (:`then`
          (set `self.NextLocationIndex` 0)
          (bind _returnvalue_2 (`|SpawnActorFromClass` "/Game/Characters/Enemy/Melee/Dog/BP_ZigZagSpline.BP_ZigZagSpline_C" (`KismetMathLibrary.MakeTransform` _returnvalue (`KismetMathLibrary.FindLookAtRotation` _returnvalue (`Actor.K2_GetActorLocation` _targetactor_2))) "AlwaysSpawn" "MultiplyWithRoot" null (`Actor.GetDistanceTo` _controllercontext _targetactor) (`Actor.K2_GetActorLocation` _targetactor) null))
          (set `self.SplineActor` _returnvalue_2)
          (message `EnemyGPInterface.Acceleration` (`Controller.K2_GetPawn` (`self.ControllerContext`))))
        (:`else`)))))

(event `self.ReceiveLatentTick`
  (params (DeltaTime :type "Float (single-precision)"))
  (bind _controllercontext (`self.ControllerContext`))
  (bind _nextlocationindex (`self.NextLocationIndex`))
  (`self.TargetActor`
    (:`then`
      (bind _splineactor (`self.SplineActor`)
        (:`then`
          (bind _spline (`/Game/Characters/Enemy/Melee/Dog/BP_ZigZagSpline.Spline` _splineactor))
          (if (<= _nextlocationindex (`SplineComponent.GetNumberOfSplinePoints` _spline)) :!label _label
            (bind _returnvalue (`SplineComponent.GetLocationAtSplinePoint` _spline _nextlocationindex "World"))
            (`AIController.K2_SetFocalPoint` _controllercontext _returnvalue)
            (`AITask_MoveTo.AIMoveTo` _controllercontext _returnvalue null
              (:`OnRequestFailed`
                (`self.FinishFail`))
              (:`OnMoveFinished`
                (`/Engine/EditorBlueprintResources/StandardMacros.IncrementInt` (`self.NextLocationIndex`)
                  (:`  `
                    (goto _label)))))
            (else
              (`Actor.K2_DestroyActor` (`self.SplineActor`))
              (`self.FinishTask` true))))
        (:`else`
          (`self.FinishFail`))))
    (:`else`
      (`self.FinishFail`))))

(fn `FinishFail`
  (message `EnemyGPInterface.ApplyNormalMovement` (`Controller.K2_GetPawn` (`self.ControllerContext`)))
  (bind _splineactor (`self.SplineActor`)
    (:`then`
      (`Actor.K2_DestroyActor` _splineactor)
      (`self.FinishTask` false))
    (:`else`)))