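; StateTree task that makes an AI pawn wander between random reachable points for a set time.
; Each AIMoveTo targets a point within Radius of the pawn's current location, so the wander area drifts with it.
; Successful moves chain while IsActive holds; a timer clears that flag, and the task succeeds once the current move completes.
; A failed move prints a message and fails the task.
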(event `self.ReceiveLatentEnterState`
  (params (Transition :type "StateTreeTransitionResult Structure (by ref)"))
  (`KismetSystemLibrary.K2_SetTimerDelegate` (delegate `Finish`) (`self.Time`))
  (`self.MoveInArea`))

(event `Finish`
  (set `self.IsActive` false))

(event `MoveInArea`
  (`|AIMoveTo` (`self.PawnContext`) (`NavigationSystemV1.K2_GetRandomReachablePointInRadius` (`Actor.K2_GetActorLocation` (`self.PawnContext`)) (`self.Radius`) null null) null
    (:`OnSuccess`
      (`self.IsActive`
        (:`then`
          (`self.MoveInArea`))
        (:`else`
          (`self.FinishTask` true))))
    (:`OnFail`
      (`KismetSystemLibrary.PrintString` "MoveArea: Failed" true true (struct :`R` 1.0 :`G` 0.010401 :`B` 0.001462 :`A` 1.0))
      (`self.FinishTask` false))))