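; StateTree task that makes an AI pawn fire from cover, extending a parent firing task.
; After a start delay, it gets the pawn's cover component and claims free space, failing the task if either step fails.
; It then switches the pawn's animation state and runs the parent fire logic after a brief pause.
; Stopping calls the parent stop, changes the animation state again and resets the free space.
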(event `self.Fire`
  (`KismetSystemLibrary.Delay` (`self.DelayStartFire`))
  (bind _contextpawn (`self.ContextPawn`)
    (:`then`
      (bind _returnvalue (message `CoverComponentInterface.GetCoverComponent` _contextpawn))
      (bind _output_get (set `self.CoverComponent` _returnvalue))
      (`/Engine/EditorBlueprintResources/StandardMacros.IsValid` _output_get
        (:`Is Valid`
          (bind _returnvalue_2 (`CoverComponent.SetFreeSpace` _output_get))
          (if _returnvalue_2
            (message `/Game/Characters/Enemy/BPI_Enemy_Animation.ChangeAnimState` (`self.ContextPawn`) "NewEnumerator4")
            (`KismetSystemLibrary.Delay` 0.2)
            (`parent.Fire`)
            (else
              (`KismetSystemLibrary.PrintString` "Failed Free Space")
              (`self.FinishTask` false))))
        (:`Is Not Valid`
          (`KismetSystemLibrary.PrintString` "Haven't cover component")
          (`self.FinishTask` false))))
    (:`else`)))

(event `self.StopFiring`
  (`parent.StopFiring`)
  (message `/Game/Characters/Enemy/BPI_Enemy_Animation.ChangeAnimState` (`self.ContextPawn`) "NewEnumerator0")
  (bind _covercomponent (`self.CoverComponent`)
    (:`then`
      (`CoverComponent.ResetFreeSpace` _covercomponent))
    (:`else`)))