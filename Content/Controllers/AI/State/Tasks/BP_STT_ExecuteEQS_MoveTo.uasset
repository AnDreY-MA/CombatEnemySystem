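; StateTree task that runs an EQS query for an AI and moves it to the resulting location or actor.
; On enter it uncovers the pawn's cover component, then tries to reserve results implementing DestinationActorInterface, failing if refused.
; When AI MoveTo finishes, it writes the target to the Destination property ref and succeeds; query or request failures fail the task.
; State completion stops active movement.
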(event `self.ReceiveLatentEnterState`
  (params (Transition :type "StateTreeTransitionResult Structure (by ref)"))
  (bind _debug (`self.Debug`))
  (bind _debug_2 (`self.Debug`))
  (bind _debug_3 (`self.Debug`))
  (`self.In Environment Query`
    (:`then`
      (`|ExecutionSequence`
        (:`then_0`
          (bind _returnvalue (message `CoverComponentInterface.GetCoverComponent` (`self.PawnContext`)))
          (`/Engine/EditorBlueprintResources/StandardMacros.IsValid` _returnvalue
            (:`Is Valid`
              (`CoverComponent.UnCover` _returnvalue))))
        (:`then_1`
          (bind (_asynctaskproxy _location _targetitem) (`RunEQSQuery_Task.RunEQSQuery_Task` (`self.ControllerContext`) (`self.In Environment Query`) (`self.EqueryConfig`) (`self.Run Mode`))
            (:`then`
              (set `self.Async Action` _asynctaskproxy))
            (:`OnSuccess`
              (set `self.TargetLocation` _location)
              (set `self.Target Item` _targetitem)
              (`|ExecutionSequence`
                (:`then_0`
                  ; Check is Destination Actor reserved
                  (bind _destinationactor (`self.CheckDestinationActor`)
                    (:`True`
                      (bind _returnvalue_2 (message `DestinationActorInterface.Reserve` _destinationactor))
                      (if _returnvalue_2
                        (`KismetSystemLibrary.PrintString` "Success Reserved")
                        (else
                          (`KismetSystemLibrary.PrintString` "Failed because point reserved" _debug_3 _debug_3 (struct :`R` 1.0 :`B` 0.040888 :`A` 1.0))
                          (`self.FinishTask` false))))))
                (:`then_1`
                  (bind _asynctaskproxy_2 (`AITask_MoveTo.AIMoveTo` (`self.ControllerContext`) (`self.TargetLocation`) (`self.Target Item`) -1.0 "Default" "Default" true (`self.Lock AILogic`))
                    (:`then`
                      (set `self.MoveTask` _asynctaskproxy_2)
                      (if (`self.Debug`)
                        (`KismetSystemLibrary.DrawDebugBox` (0.0 0.0 0.0) (`self.TargetLocation`) (struct :`B` 1.0 :`A` 1.0) (struct) 3.0 2.0)))
                    (:`OnRequestFailed`
                      (`self.BroadcastDelegate` (`self.OnFailed`))
                      (`KismetSystemLibrary.PrintString` "Failed Move" _debug_2 _debug_2 (struct :`R` 1.0 :`B` 0.040888 :`A` 1.0))
                      (`self.FinishTask` false))
                    (:`OnMoveFinished`
                      (`self.Target Item`
                        (:`then`
                          (bind _reference (`|StateTreeBlueprintPropertyRef` (`self.Destination`))
                            (:`Succeeded`
                              (`|VariableSetRef` _reference (`self.Target Item`)))
                            (:`Failed`
                              _)))
                        (:`else`
                          _))
                      (`self.BroadcastDelegate` (`self.OnSuccess`))
                      (`self.FinishTask` true))))))
            (:`OnFailed`
              (`self.BroadcastDelegate` (`self.OnFailed`))
              (`KismetSystemLibrary.PrintString` "Failed Query" _debug _debug (struct :`R` 1.0 :`G` 0.033427 :`A` 1.0))
              (`self.FinishTask` false))))))
    (:`else`
      (`self.FinishTask` false))))

(event `self.ReceiveStateCompleted`
  (params (CompletionStatus :type "EStateTreeRunStatus Enum" :default "Running") (CompletedActiveStates :type "StateTreeActiveStates Structure"))
  (`parent.ReceiveStateCompleted` CompletionStatus CompletedActiveStates)
  (bind _movetask (`self.MoveTask`)
    (:`then`
      (message `NavMovementInterface.StopActiveMovement` _movetask)
      (set `self.MoveTask` null))
    (:`else`)))