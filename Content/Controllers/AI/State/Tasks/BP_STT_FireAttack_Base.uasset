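; Base StateTree task that makes an AI pawn fire at a target actor, gated by the AI Director's attack-level reservation.
; On enter it reserves the level, then line-traces on Visibility from just above the pelvis to confirm nothing blocks the target.
; It fires and succeeds after the attack-speed delay, or fails if reservation or trace fails.
; State completion stops firing and releases the reservation.
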(event `self.ReceiveLatentEnterState`
  (params (Transition :type "StateTreeTransitionResult Structure (by ref)"))
  (bind _returnvalue (`DirectorCombatAIComponent.ReserveLevelAttack` (`CombatAIFunctionLibrary.GetDirectorAI`) (`self.ContextController`) (`self.LevelAttack`)))
  (if _returnvalue
    (`self.Fire`)
    (else
      (`KismetSystemLibrary.PrintString` "Attack has be reserved" true true (struct :`R` 1.0 :`G` 0.32581 :`B` 0.00209 :`A` 1.0) 3.0)
      (`self.FinishTask` false))))

(event `Fire`
  (if (`self.CheckBlocking`)
    (message `CombatEnemyInterface.StartFire` (`self.ContextPawn`) (`Actor.K2_GetActorLocation` (`self.TargetActor`)))
    (`KismetSystemLibrary.Delay` (`self.AttackSpeed`))
    (`self.FinishTask` true)
    (else
      (`KismetSystemLibrary.PrintString` "Fire is blocking")
      (`self.FinishTask` false))))

(event `StopFiring`
  (message `CombatEnemyInterface.StopFiring` (`self.ContextPawn`))
  (`DirectorCombatAIComponent.ReleaseLevelAttack` (`CombatAIFunctionLibrary.GetDirectorAI`) (`self.ContextController`) (`self.LevelAttack`)))

(event `self.ReceiveStateCompleted`
  (params (CompletionStatus :type "EStateTreeRunStatus Enum" :default "Running") (CompletedActiveStates :type "StateTreeActiveStates Structure"))
  (switch `EStateTreeRunStatus` CompletionStatus
    (:`Stopped`
      _)
    (:`Succeeded`
      _)
    (:`Failed`
      _))
  (`self.StopFiring`))

(fn `CheckBlocking`
  (returns (CanFire :type Boolean))
  (bind _contextpawn (`self.ContextPawn`)
    (:`then`
      (bind _returnvalue (* (`Actor.GetActorUpVector` _contextpawn) 10.0))
      (bind (_outhit _returnvalue_2) (`KismetSystemLibrary.LineTraceSingle` (+ (`SceneComponent.GetSocketLocation` (`Character.Mesh` _contextpawn) "pelvis") _returnvalue) (+ _returnvalue (`Actor.K2_GetActorLocation` (`self.TargetActor`))) "TraceTypeQuery1" false (`|MakeArray` (`self.ContextPawn`) :!type "Actor Object Reference")))
      (if _returnvalue_2
        (bind _targetactor (`self.TargetActor`)
          (:`then`
            (if (== (`.HitActor` (`GameplayStatics.BreakHitResult` _outhit)) _targetactor)
              (return true)
              (else
                _)))
          (:`else`
            _)))
      (return false))
    (:`else`
      (return false))))