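; BP_STT_Strafe is a State Tree task that makes an AI strafe around its target.
; On entering the state, it focuses the controller on the target actor and runs an environment query for a location around it, picking randomly from the best 25 percent.
; The AI moves there, with a debug box drawn at the spot.
; The task succeeds when the move finishes and fails if the query or move request fails.
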(event `self.ReceiveLatentEnterState`
  (params (Transition :type "StateTreeTransitionResult Structure (by ref)"))
  (bind _returnvalue (message `EnemyControlInterface.GetTargetActor` (`self.ControllerContext`)))
  (`/Engine/EditorBlueprintResources/StandardMacros.IsValid` _returnvalue
    (:`Is Valid`
      (`AIController.K2_SetFocus` (`self.ControllerContext`) _returnvalue)
      (bind _location (`RunEQSQuery_Task.FindAroundTargetLocation_Task` (`self.ControllerContext`) (`self.In Environment Query`) "RandomBest25Pct")
        (:`OnSuccess`
          (`AITask_MoveTo.AIMoveTo` (`self.ControllerContext`) _location null 5.0 "Default" "Disable"
            (:`then`
              (`KismetSystemLibrary.DrawDebugBox` _location (5.0 5.0 5.0) (struct :`R` 0.345457 :`B` 1.0 :`A` 1.0) (struct) 2.0))
            (:`OnRequestFailed`
              (`self.FinishTask` false))
            (:`OnMoveFinished`
              (`self.FinishTask` true))))
        (:`OnFailed`
          (`self.FinishTask` false))))))