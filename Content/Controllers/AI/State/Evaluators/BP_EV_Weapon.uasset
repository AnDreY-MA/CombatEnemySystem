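; A StateTree evaluator that exposes the AI pawn's weapon component and current ammo to the tree.
; On tree start it waits a tick, caches the pawn's WeaponComponent and initial ammo, and binds to its ammo-changed event.
; Each ammo change updates the stored count and sends an Events.AI.Reload event into the StateTree, regardless of the new amount.
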(event `self.ReceiveTreeStart`
  (bind _returnvalue (`Actor.GetComponentByClass` (`self.ContextPawn`) "/Game/ActorComponents/WeaponComponent.WeaponComponent_C"))
  (`KismetSystemLibrary.DelayUntilNextTick`)
  (`/Engine/EditorBlueprintResources/StandardMacros.IsValid` _returnvalue
    (:`Is Valid`
      (bind _output_get (set `self.WeaponComponent` _returnvalue))
      (set `self.CurrentAmmo` (`/Game/ActorComponents/WeaponComponent.GetAmmo` _output_get))
      (add `/Game/ActorComponents/WeaponComponent.OnAmmoChanged` (`self.WeaponComponent`) (`|CreateDelegate` :!event `OnAmmoChanged`)))))

(event `OnAmmoChanged`
  (params (CurrentAmount :type "Integer (by ref)"))
  (set `self.CurrentAmmo` CurrentAmount)
  (`self.SendEvent` (make `StateTreeEvent` (struct :`TagName` "Events.AI.Reload"))))